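; Game instance for the Runner game that manages the record save and music volume across the session.
; On Init it checks Android storage permission, requesting it if missing, then loads or creates the BP_RunnerSaveGame object.
; Save and load functions expose the game record, with saving reloading the object if invalid.
; Init also sets the base sound mix and applies music volume through a sound class override.
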(event Custom|AndroidPermissionGranted
  (params (Permissions :type Array%20of%20Strings) (GrantResults :type Array%20of%20Booleans))
  ;[0.5997 1 0.5943] SaveGame Initialization
  (if (Utilities|Array|Get(acopy) GrantResults)
    (CallFunction|LoadRunnerGameData)))

(event Custom|UpdateSoundSetup
  (params (InSoundClass :type Sound%20Class%20Object%20Reference) (Volume :type Float%20%28single-precision%29))
  ;[0.5354 0.6305 1] Sound Setup
  (bind _output_get (Variables|Default|SetSoundMusicVolume Volume))
  (Audio|SetSoundMixClassOverride "/Game/Runner/Blueprints/Sounds/SM_Mix.SM_Mix" InSoundClass _output_get 1.0 0.0 true))

(event EventInit
  (Utilities|FlowControl|Sequence
    (:then_0
      ;[0.5997 1 0.5943] SaveGame Initialization
      (bind _returnvalue (Class|AndroidPermissionFunctionLibrary|CheckPermission "android.permission.WRITE_EXTRNAL_STORAGE"))
      (if _returnvalue
        (CallFunction|LoadRunnerGameData)
        (else
          (bind _returnvalue_2 (Class|AndroidPermissionFunctionLibrary|AcquirePermissions (Utilities|Array|MakeArray "android.permission.WRITE_EXTRNAL_STORAGE" "android.permission.READ_EXTRNAL_STORAGE")))
          (EventDispatchers|BindEventtoOnPermissionsGrantedDynamicDelegate _returnvalue_2 (delegate Custom|AndroidPermissionGranted)))))
    (:then_1
      ;[0.5354 0.6305 1] Sound Setup
      (Class|GameplayStatics|SetBaseSoundMix "/Game/Runner/Blueprints/Sounds/SM_Mix.SM_Mix")
      (CallFunction|UpdateSoundSetup "/Game/Runner/Blueprints/Sounds/SC_Music.SC_Music" (Variables|Default|GetSoundMusicVolume)))))

(fn LoadRunnerGameData
  (bind _returnvalue (SaveGame|DoesSaveGameExist (Variables|Default|GetSaveSlotName)))
  (if _returnvalue
    (bind _returnvalue_2 (SaveGame|LoadGamefromSlot (Variables|Default|GetSaveSlotName)))
    (bind _asbp_runner_save_game (Utilities|Casting|CastToBP_RunnerSaveGame _returnvalue_2))
    (bind _output_get (Variables|Default|SetRunnerSaveGame _asbp_runner_save_game))
    (return (Variables|/Game/Runner/Blueprints/BP_RunnerSaveGame.BP_RunnerSaveGame_C|GetGameRecord _output_get))
    (else
      (bind _returnvalue_3 (SaveGame|CreateSaveGameObject "/Game/Runner/Blueprints/BP_RunnerSaveGame.BP_RunnerSaveGame_C"))
      (Variables|Default|SetRunnerSaveGame _returnvalue_3)
      (return 0))))

(fn SaveRunnerGameData
  (params (NewRecord :type Integer))
  (bind _runnersavegame (Variables|Default|GetRunnerSaveGame)
    (:then
      _)
    (:else
      (CallFunction|LoadRunnerGameData)))
  (Variables|/Game/Runner/Blueprints/BP_RunnerSaveGame.BP_RunnerSaveGame_C|SetGameRecord _runnersavegame NewRecord)
  (bind _returnvalue (SaveGame|SaveGametoSlot (Variables|Default|GetRunnerSaveGame) (Variables|Default|GetSaveSlotName)))
  (return _returnvalue))