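; Score pickup for the runner game, a child pickup actor that adds its value to the player's score when collected.
; Pickup passes the score value and the character's score coefficient to BP_CoreGM, then calls the parent logic that destroys the actor.
; When a runner character with an active magnet enters the sphere, a timeline lerps the pickup from its start position to the player's current location.
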(event OnComponentBeginOverlap(Sphere)
  (params (OverlappedComponent :type Primitive%20Component%20Object%20Reference) (OtherActor :type Actor%20Object%20Reference) (OtherComp :type Primitive%20Component%20Object%20Reference) (OtherBodyIndex :type Integer) (bFromSweep :type Boolean) (SweepResult :type Hit%20Result%20Structure%20%28by%20ref%29))
  (bind _asbp_runner_character (Utilities|Casting|CastToBP_RunnerCharacter OtherActor))
  (if (Variables|/Game/ThirdPersonBP/Blueprints/BP_RunnerCharacter.BP_RunnerCharacter_C|GetbMagnetActive _asbp_runner_character)
    (Variables|Default|SetStartPosition (Transformation|GetActorLocation))
    (bind _lerpalpha (Timeline|MagnetPickups PlayFromStart)
      (:Update
        (Transformation|SetActorLocation (Math|Vector|MakeVector (.x (Math|Vector|Lerp(Vector) (Variables|Default|GetStartPosition) (Transformation|GetActorLocation (Game|GetPlayerCharacter 0)) _lerpalpha)) (.y (Math|Vector|Lerp(Vector) (Variables|Default|GetStartPosition) (Transformation|GetActorLocation (Game|GetPlayerCharacter 0)) _lerpalpha)) (.z (Math|Vector|Lerp(Vector) (Variables|Default|GetStartPosition) (Transformation|GetActorLocation (Game|GetPlayerCharacter 0)) _lerpalpha))) false false)))))

(event EventBeginPlay
  (|CallParentFunction) ; This node is disabled and will not be called.\nDrag off pins to build functionality.
)

(event Collision|EventActorBeginOverlap
  (params (OtherActor :type Actor%20Object%20Reference))
  (|CallParentFunction OtherActor) ; This node is disabled and will not be called.\nDrag off pins to build functionality.
)

(event EventTick
  (params (DeltaSeconds :type Float%20%28single-precision%29))
  (|CallParentFunction DeltaSeconds))

(fn ConstructionScript
  (|CallParentFunction))

(fn Pickup
  (params (Character :type BP%20Runner%20Character%20Object%20Reference))
  (bind _asbp_core_gm (Utilities|Casting|CastToBP_CoreGM (Game|GetGameMode)))
  (Default|UpdatePlayerScore _asbp_core_gm (Variables|Setup|GetScoreValue) (Variables|/Game/ThirdPersonBP/Blueprints/BP_RunnerCharacter.BP_RunnerCharacter_C|GetPlayerScoreCoefficient Character))
  ;[1 1 1] Parent logic with Destroy
  (|CallParentFunction Character))