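; BP_PickupActorBase is the base actor for pickups in the runner game, collected when a BP_RunnerCharacter overlaps its Model component.
; The overlap passes the character to Pickup, which only destroys the actor in this base version.
; On BeginPlay, the HeightLerp timeline offsets Z from the spawn location if Bounce is set.
; A fixed delay also destroys the actor, so uncollected pickups clean themselves up.
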(event OnComponentBeginOverlap(Model)
  (params (OverlappedComponent :type Primitive%20Component%20Object%20Reference) (OtherActor :type Actor%20Object%20Reference) (OtherComp :type Primitive%20Component%20Object%20Reference) (OtherBodyIndex :type Integer) (bFromSweep :type Boolean) (SweepResult :type Hit%20Result%20Structure%20%28by%20ref%29))
  ;[1 0.9127 0.02884] Check Character
  (bind _asbp_runner_character (Utilities|Casting|CastToBP_RunnerCharacter OtherActor))
  ;[0.1456 1 0.3592] Call Pickup (Logic + VFX + SFX) + Destroy
  (CallFunction|Pickup _asbp_runner_character))

(event EventBeginPlay
  (Variables|Default|SetActorSpawnLocation (Transformation|GetActorLocation))
  (Utilities|FlowControl|Sequence
    (:then_0
      (if (Variables|Default|GetbBounce)
        (bind _z_value (Timeline|HeightLerp PlayFromStart)
          (:Update
            (Transformation|SetActorLocation (Math|Vector|MakeVector (.x (Variables|Default|GetActorSpawnLocation)) (.y (Variables|Default|GetActorSpawnLocation)) (+ (.z (Variables|Default|GetActorSpawnLocation)) _z_value)) false false)))))
    (:then_1
      ;[1 0 0.02448] Delay for Delete
      (Utilities|FlowControl|Delay 2e+01)
      (Actor|DestroyActor))))

(event Collision|EventActorBeginOverlap
  (params (OtherActor :type Actor%20Object%20Reference)))

(event EventTick
  (params (DeltaSeconds :type Float%20%28single-precision%29)))

(fn ConstructionScript)

(fn Pickup
  (params (Character :type BP%20Runner%20Character%20Object%20Reference))
  ;[1 0.02604 0.02604] Destroy
  (Actor|DestroyActor))