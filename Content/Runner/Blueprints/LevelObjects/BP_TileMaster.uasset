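; Runner track tile that randomly populates itself with obstacles and pickups, then extends the track as the player runs.
; On BeginPlay, three lane points roll for walls or powerups, halving obstacle odds after each wall and allowing one powerup.
; Score pickups and an occasional box land at grid-snapped random points inside a volume.
; The trigger makes BP_CoreGM spawn the next tile and raise player speed, then destroys this tile after a delay.
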(event OnComponentBeginOverlap(Trigger)
  (params (OverlappedComponent :type Primitive%20Component%20Object%20Reference) (OtherActor :type Actor%20Object%20Reference) (OtherComp :type Primitive%20Component%20Object%20Reference) (OtherBodyIndex :type Integer) (bFromSweep :type Boolean) (SweepResult :type Hit%20Result%20Structure%20%28by%20ref%29))
  (Utilities|Casting|CastToBP_RunnerCharacter OtherActor)
  (bind _asbp_core_gm (Utilities|Casting|CastToBP_CoreGM (Game|GetGameMode)))
  (Default|SpawnNewTile _asbp_core_gm)
  (bind _result (Math|Integer|IncrementInt (Variables|/Game/Runner/Blueprints/BP_CoreGM.BP_CoreGM_C|GetTilesLeftBehind _asbp_core_gm))
    (:%20%20
      (Utilities|FlowControl|Sequence
        (:then_0
          (Utilities|FlowControl|Delay 1.0)
          (Actor|DestroyActor))
        (:then_2
          (Default|UpdatePlayerSpeed _asbp_core_gm 1e+01))))))

(event Custom|Spawn
  (bind _walltypes (Variables|Default|GetWallTypes))
  (bind _poweruptypes (Variables|Default|GetPowerupTypes))
  (for (_ _array_index) (Variables|Default|GetSpawnLocations)
    (switch int (Math|Random|RandomIntegerinRange 0 2)
      (:Default
        ;[1 1 1] Spawn Wall
        (if (> (Utilities|Array|Length _walltypes) 0) :!label _label
          (if (Math|Integer|InRange(Integer) (Math|Random|RandomIntegerinRange 0 100) 0 (Variables|Default|GetObstacleSpawnRate))
            (Game|SpawnActorfromClass (Utilities|Array|Get(acopy) _walltypes (Math|Random|RandomIntegerinRange 0 (Utilities|Array|LastIndex _walltypes))) (Math|Transform|MakeTransform (Utilities|Array|Get(acopy) (Variables|Default|GetSpawnLocations) _array_index) "0, 0, 0" "1,1,1") "Undefined" 0 0)
            (Variables|Default|SetObstacleSpawnRate (/ (Variables|Default|GetObstacleSpawnRate) 2)))))
      (:0
        (goto _label))
      (:2
        ;[1 1 1] Spawn Ramp
        (if (> (Utilities|Array|Length _poweruptypes) 0)
          (if (Math|Integer|InRange(Integer) (Math|Random|RandomIntegerinRange 0 100) 0 (Variables|Default|GetBonusSpawnRate))
            (Game|SpawnActorfromClass (Utilities|Array|Get(acopy) _poweruptypes (Math|Random|RandomIntegerinRange 0 (Utilities|Array|LastIndex _poweruptypes))) (Math|Transform|MakeTransform (Utilities|Array|Get(acopy) (Variables|Default|GetSpawnLocations) _array_index) "0, 0, 0" "1,1,1") "Undefined" 0 0)
            (bind _asbp_core_gm (Utilities|Casting|CastToBP_CoreGM (Game|GetGameMode)))
            (Default|UpdateBonusSpawnRate _asbp_core_gm true)
            (Variables|Default|SetBonusSpawnRate 0)))))))

(event EventBeginPlay
  (bind _pickupspawnvolume (Variables|Default|GetPickupSpawnVolume))
  (bind _pickupspawnvolume_2 (Variables|Default|GetPickupSpawnVolume))
  (bind (_origin _boxextent) (Collision|GetComponentBounds _pickupspawnvolume))
  (bind (_origin_2 _boxextent_2) (Collision|GetComponentBounds _pickupspawnvolume_2))
  (bind _returnvalue (Math|Random|RandomPointinBoundingBox _origin _boxextent))
  (bind _returnvalue_2 (Math|Random|RandomPointinBoundingBox _origin_2 _boxextent_2))
  (bind (_x _y) (Math|Vector|BreakVector _returnvalue))
  (bind (_x_2 _y_2) (Math|Vector|BreakVector _returnvalue_2))
  (CallFunction|Spawn)
  (Utilities|FlowControl|Sequence
    (:then_0
      (for _index (range 0 (Math|Random|RandomIntegerinRange 0 3))
        (Game|SpawnActorfromClass "/Game/Runner/Blueprints/PickupObjects/BP_PickupScoreActor.BP_PickupScoreActor_C" (Math|Transform|MakeTransform (Math|Vector|MakeVector (Math|Float|SnapToGrid(Float) _x 5e+01) (Math|Float|SnapToGrid(Float) _y 2e+02) (+ (.Z (Math|Vector|BreakVector _origin)) 4e+01)) "0, 0, 0" "1,1,1") "Undefined" 0 1 0)))
    (:then_1
      (if (Math|Integer|InRange(Integer) (Math|Random|RandomIntegerinRange 0 100) 0 (Variables|Default|GetObstacleSpawnRate))
        (Game|SpawnActorfromClass "/Game/Runner/Blueprints/LevelObjects/BP_ObstacleBoxActor.BP_ObstacleBoxActor_C" (Math|Transform|MakeTransform (Math|Vector|MakeVector (Math|Float|SnapToGrid(Float) _x_2 5e+01) (Math|Float|SnapToGrid(Float) _y_2 2e+02) (- (.Z (Math|Vector|BreakVector _origin_2)) (.Z (Math|Vector|BreakVector _boxextent_2)))) "0, 0, 0" "1,1,1") "Undefined" 0 0)))))

(event Collision|EventActorBeginOverlap
  (params (OtherActor :type Actor%20Object%20Reference)))

(event EventTick
  (params (DeltaSeconds :type Float%20%28single-precision%29)))

(fn ConstructionScript
  (CallFunction|SetupSpawnPoints)
  (CallFunction|SpawnObstacle))

(fn SetupSpawnPoints
  (Variables|Default|SetSpawnLocations (Utilities|Array|MakeArray (Transformation|GetWorldLocation (Variables|Default|GetLine1)) (Transformation|GetWorldLocation (Variables|Default|GetLine2)) (Transformation|GetWorldLocation (Variables|Default|GetLine3)))))

(fn SpawnObstacle)