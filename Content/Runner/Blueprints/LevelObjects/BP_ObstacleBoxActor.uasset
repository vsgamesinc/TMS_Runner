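; BP_ObstacleBoxActor is an obstacle box in the runner game that costs the player score when hit.
; When a BP_RunnerCharacter overlaps it, HitObstacle subtracts ScoreDebuff through BP_CoreGM's UpdatePlayerScore, provided the character is not dead.
; BreakObstacle then destroys the actor, whether or not the character was alive.
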(event Custom|BreakObstacle
  (Actor|DestroyActor))

(event EventBeginPlay
  (|CallParentFunction))

(event Collision|EventActorBeginOverlap
  (params (OtherActor :type Actor%20Object%20Reference))
  (bind _asbp_runner_character (Utilities|Casting|CastToBP_RunnerCharacter OtherActor))
  (CallFunction|HitObstacle _asbp_runner_character)
  (CallFunction|BreakObstacle))

(event EventTick
  (params (DeltaSeconds :type Float%20%28single-precision%29))
  (|CallParentFunction DeltaSeconds) ; This node is disabled and will not be called.\nDrag off pins to build functionality.
)

(fn ConstructionScript
  (|CallParentFunction))

(fn HitObstacle
  (params (Character :type BP%20Runner%20Character%20Object%20Reference))
  (if (not (Variables|/Game/ThirdPersonBP/Blueprints/BP_RunnerCharacter.BP_RunnerCharacter_C|GetisDead Character))
    (bind _asbp_core_gm (Utilities|Casting|CastToBP_CoreGM (Game|GetGameMode)))
    (Default|UpdatePlayerScore _asbp_core_gm (- 0 (Variables|Default|GetScoreDebuff)) 1.0))
  (return false))