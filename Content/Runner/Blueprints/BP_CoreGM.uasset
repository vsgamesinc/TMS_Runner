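; Game mode for an endless runner that spawns track tiles, tracks score and adjusts player speed.
; Random tiles chain through each SnapPoint with obstacle and bonus rates passed at spawn; the first tile also caches three lane Y positions.
; BeginPlay pre-spawns tiles with an obstacle-wall-free start, then sets up HUD, fog and music.
; Bonus rate can drop to zero and climbs back per spawned tile; game end switches to death music.
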(event Custom|SpawnNewTile
  (params (ObstacleWallSpawnRateOverride :type Integer))
  (bind _leveltiles (Variables|Spawn|GetLevelTiles))
  (bind _returnvalue (Game|SpawnActorfromClass (Utilities|Array|Get(acopy) _leveltiles (Math|Random|RandomIntegerinRange 0 (Utilities|Array|LastIndex _leveltiles))) (Math|Transform|MakeTransform (Variables|Spawn|GetNextTilePosition)) "Undefined" self (select (< ObstacleWallSpawnRateOverride 0) (Variables|Spawn|GetObstacleWallSpawnRate) ObstacleWallSpawnRateOverride) (Variables|Spawn|GetObstacleRampSpawnRate) (Variables|Spawn|GetObstacleBoxSpawnRate) (Variables|Spawn|GetBonusSpawnRateOverride) 0))
  (Variables|Spawn|SetNextTilePosition (Transformation|GetWorldLocation (Variables|/Game/Runner/Blueprints/LevelObjects/BP_TileMaster.BP_TileMaster_C|GetSnapPoint _returnvalue)))
  (CallFunction|UpdateBonusSpawnRate false)
  ;[0.5641 1 0.4951] Update Lines
  (if (not (Variables|Game|GetbLinesReady))
    (Variables|Setup|SetLinesY (Utilities|Array|MakeArray (.Y (Math|Vector|BreakVector (Transformation|GetWorldLocation (Variables|/Game/Runner/Blueprints/LevelObjects/BP_TileMaster.BP_TileMaster_C|GetLine1 _returnvalue)))) (.Y (Math|Vector|BreakVector (Transformation|GetWorldLocation (Variables|/Game/Runner/Blueprints/LevelObjects/BP_TileMaster.BP_TileMaster_C|GetLine2 _returnvalue)))) (.y (Transformation|GetWorldLocation (Variables|/Game/Runner/Blueprints/LevelObjects/BP_TileMaster.BP_TileMaster_C|GetLine3 _returnvalue)))))
    (Variables|Game|SetbLinesReady true)))

(event Custom|SoundEndGame
  (Audio|Components|Audio|FadeOut (Variables|Default|GetGameMusic) 1.0 0.0 "Linear" :!class /Script/Engine.AudioComponent)
  (Audio|Components|Audio|Play (Variables|Default|GetDeathMusic) 0.0))

(event EventBeginPlay
  (Utilities|FlowControl|Sequence
    (:then_0
      ;[1 1 1] Level Spawn Preprocessing
      (Variables|Spawn|SetBonusSpawnRateOverride (Variables|Spawn|GetBonusSpawnRate))
      (for _index (range 0 (- (Variables|Spawn|GetTIleSpawnCount) 1))
        (CallFunction|SpawnNewTile (select (< _index (- (Variables|Spawn|GetTIleSpawnClearCount) 1)) 0 -1))))
    (:then_1
      (bind _returnvalue (UserInterface|CreateWidget "/Game/Runner/GUI/WBP_GameHUD.WBP_GameHUD_C" (Game|GetPlayerController 0)))
      (bind _output_get (Variables|Default|SetHUD _returnvalue))
      (UserInterface|Viewport|AddtoViewport _output_get 0))
    (:then_2
      (Rendering|Material|SetScalarParameterValue "/Game/Runner/Materials/MPC_GameParams.MPC_GameParams" "Fog_Distance" 8e+03 :!class /Script/Engine.KismetMaterialLibrary))
    (:then_3
      (Audio|Components|Audio|Play (Variables|Default|GetGameMusic) 0.0))))

(fn ConstructionScript)

(fn GetCurrentLineY
  (return (.y (Variables|Spawn|GetNextTilePosition))))

(fn GetLinesY
  (return (Variables|Setup|GetLinesY)))

(fn GetPlayerScore
  (return (Variables|Game|GetPlayerScore)))

(fn UpdatePlayerScore
  (params (Value :type Integer) (Coefficient :type Float%20%28single-precision%29))
  (bind _output_get (Variables|Game|SetPlayerScore (Math|Integer|Clamp(Integer) (+ (Variables|Game|GetPlayerScore) (Math|Float|Truncate (* Value Coefficient))) 0 (+ (Variables|Game|GetPlayerScore) (Math|Float|Truncate (* Value Coefficient))))))
  (return _output_get))

(fn UpdatePlayerSpeed
  (params (Coefficient :type Float%20%28single-precision%29))
  (bind _returnvalue (Game|GetPlayerCharacter 0))
  (bind _charactermovement (Variables|/Script/Engine.Character|GetCharacterMovement _returnvalue))
  (Variables|/Script/Engine.CharacterMovementComponent|SetMaxWalkSpeed _charactermovement (Math|Float|Clamp(Float) (+ (Variables|/Script/Engine.CharacterMovementComponent|GetMaxWalkSpeed _charactermovement) Coefficient) 6e+02 (Variables|Rules|GetMaximumSpeed))))

(fn UpdateBonusSpawnRate
  (params (SetToZero :type Boolean))
  (if SetToZero
    (Variables|Spawn|SetBonusSpawnRateOverride 0)
    (else
      (Variables|Spawn|SetBonusSpawnRateOverride (Math|Integer|Clamp(Integer) (+ (Variables|Spawn|GetBonusSpawnRateOverride) 1) 0 (Variables|Spawn|GetBonusSpawnRate))))))